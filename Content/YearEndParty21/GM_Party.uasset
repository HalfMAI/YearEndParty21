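; Game mode for a year-end party prize draw, handling server requests, draw animations and result widgets.
; A fresh BP_HttpHandle serves each request; timer-drained queues fetch player pools and images, caching textures by URL.
; BPO_Drawer stores draw data; animation-status callbacks start or stop the popup, BP_DrawerPlayers effects and result screen.
; Startup and polling are disconnected, and the start animation uses a test spawn from a hard-coded pool.
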(event Custom|Test_ShowAnimateWithDrawing
  (params (PoolID :type String) (AwardName :type String) (DrawNum :type Integer))
  (CallFunction|RequestStartDraw PoolID AwardName DrawNum))

(event Custom|TestingGet
  (params (Duration :type Float%20%28single-precision%29))
  (bind _g_spawnfx (Variables|Default|Getg_SpawnFX))
  (Utilities|FlowControl|Delay Duration)
  (Default|StartSpawn _g_spawnfx (.PoolPlayers (Utilities|Struct|BreakStruct_Pool (.Value (Utilities|Map|Find (Variables|/Game/YearEndParty21/Blueprints/DrawerHttpHandler/BPO_Drawer.BPO_Drawer_C|Getg_PlayerList (Variables|Default|Getg_Drawer)) "普通奖品用户池-员工名单")))))
  (Utilities|FlowControl|Delay 1.0)
  (Default|PlayEndAnimtion _g_spawnfx))

(event Custom|OnStartAnimation
  (params (PoolID :type String) (AwardName :type String) (LastDrawNum :type Integer) (PlayersInfo :type Array%20of%20Struct%20Player%20Structures))
  (if (not (Variables|Default|GetIsAlreadyPlayingAnimation?))
    (CallFunction|ResetAnimationStatus)
    (Variables|Default|SetIsAlreadyPlayingAnimation? true)
    (bind _savedlastdrawawardinfo (Default|SetupLastDrawInfo (Variables|Default|Getg_Drawer) PoolID AwardName LastDrawNum PlayersInfo (Variables|Http|Getg_DownloadTex2d)))
    (Utilities|FlowControl|Sequence
      (:then_0
        (CallFunction|ShowHideUI (Variables|Default|GetRef_WBP_AwardList) false false)
        (bind _returnvalue (UserInterface|CreateWidget "/Game/YearEndParty21/WBP/WBP_StartDrawPopUp.WBP_StartDrawPopUp_C"))
        (UserInterface|Viewport|AddtoViewport _returnvalue 0)
        (Default|PlayAnimationAnDestory _returnvalue (.AwardName (Utilities|Struct|BreakStruct_Award _savedlastdrawawardinfo)) (.AwardImgTex2d (Utilities|Struct|BreakStruct_Award _savedlastdrawawardinfo))))
      (:then_1
        (CallFunction|TestingGet 0.0)))))

(event Custom|OnStopAnimation
  (bind _g_drawer (Variables|Default|Getg_Drawer))
  (bind _g_lastdrawedawardinfo (Variables|/Game/YearEndParty21/Blueprints/DrawerHttpHandler/BPO_Drawer.BPO_Drawer_C|Getg_LastDrawedAwardInfo _g_drawer))
  (if (Variables|Default|GetIsAlreadyPlayingAnimation?)
    (CallFunction|ResetAnimationStatus)
    (Variables|Default|SetIsAlreadyPlayingAnimation? false)
    (CallFunction|DrawedInfoCallbackandShowResultWBP (.poolid _g_lastdrawedawardinfo) (.awardname _g_lastdrawedawardinfo) (Variables|/Game/YearEndParty21/Blueprints/DrawerHttpHandler/BPO_Drawer.BPO_Drawer_C|Getg_LastDrawNum _g_drawer) (Variables|/Game/YearEndParty21/Blueprints/DrawerHttpHandler/BPO_Drawer.BPO_Drawer_C|Getg_LastDrawedPlayerInfo _g_drawer))
    (CallFunction|ShowHideUI (Variables|Default|GetRef_WBP_AwardList) false false)))

(event Custom|tmpCheckShouldPlayAnimation
  ;[1 1 1] Loop Request Animation Status
  (CallFunction|RequestSholudPlayAnimation?))

(event EventBeginPlay)

(event Custom|RequestAwardsInfo
  (params (IsCallUI? :type Boolean))
  ;[1 1 1] AwardsInfo
  (Http|RequestAwardsInfoFunc (delegate Custom|OnAwardsInfoCallback)))

(event Custom|RequestPoolInfo
  (params (PoolID :type String) (CallUI? :type Boolean))
  ;[1 1 1] PoolInfo
  (Http|RequestPoolInfoFunc PoolID (delegate Custom|OnPoolInfoCallback)))

(event Custom|PoolRequestQueue
  (bind _tmppoolrequestqueue (Variables|Default|GettmpPoolRequestQueue))
  (bind _output (Utilities|Array|Get(acopy) _tmppoolrequestqueue))
  ;[1 1 1] RequestPoolQueue
  (if (<= (Utilities|Array|Length _tmppoolrequestqueue) 0)
    (Utilities|FlowControl|Delay 0.2)
    (Utilities|Time|ClearandInvalidateTimerbyHandle (stale Custom|RequestPoolQueue _returnvalue))
    (Utilities|FlowControl|DoOnce false) ; enters at Reset
    (else
      (CallFunction|RequestPoolInfo _output false)
      (Utilities|Array|RemoveItem _tmppoolrequestqueue _output))))

(event Custom|RequestImageQueue
  (params (ImgURL :type String%20%28by%20ref%29))
  ;[1 1 1] RequestImgQueue
  (Utilities|FlowControl|Sequence
    (:then_0
      (Utilities|Array|AddUnique (Variables|Default|GettmpImgDownQueue) ImgURL))
    (:then_1
      (Utilities|FlowControl|DoOnce false
        (:Completed
          (bind _returnvalue (Utilities|Time|SetTimerbyEvent (delegate Custom|ImgQueueEvent) 0.05 true)))))))

(event Custom|ImgQueueEvent
  (bind _tmpimgdownqueue (Variables|Default|GettmpImgDownQueue))
  (bind _output (Utilities|Array|Get(acopy) _tmpimgdownqueue))
  ;[1 1 1] RequestImgQueue
  (for _index (range 0 10)
    (if (<= (Utilities|Array|Length _tmpimgdownqueue) 0)
      (Utilities|FlowControl|Delay 0.2)
      (Utilities|Time|ClearandInvalidateTimerbyHandle (stale Custom|RequestImageQueue _returnvalue))
      (Utilities|FlowControl|DoOnce false) ; enters at Reset
      (else
        (CallFunction|RequestImage _output self)
        (Utilities|Array|RemoveItem _tmpimgdownqueue _output)))))

(event Custom|RequestSholudPlayAnimation?
  ;[1 1 1] RequestPlayAnimation
  (Http|RequesCheckAnimationStatusFunc (delegate Custom|CheckAniStatusCallback)))

(event Custom|CheckAniStatusCallback
  (params (IsShouldStartAnimation? :type Boolean) (DrawPoolID :type String) (DrawAwardName :type String) (DrawNum :type Integer) (DrawedPlayers :type Array%20of%20Struct%20Player%20Structures))
  ;[1 1 1] RequestPlayAnimation
  (if IsShouldStartAnimation?
    (CallFunction|OnStartAnimation DrawPoolID DrawAwardName DrawNum DrawedPlayers)
    (Development|PrintString "AnimationTrue" true true "(R=1.000000,G=0.000000,B=0.003472,A=1.000000)")
    (else
      (CallFunction|OnStopAnimation)
      (Development|PrintString "AnimationFalse" true true "(R=1.000000,G=0.000000,B=0.823312,A=1.000000)"))))

(event Custom|RequestStartDraw
  (params (PoolID :type String) (AwardName :type String) (DrawNum :type Integer))
  ;[1 1 1] StartDraw
  (Http|RequestStartDrawFunc PoolID AwardName DrawNum (delegate Custom|OnDrawedInfoCallback)))

(event Custom|RequestImage
  (params (url :type String) (TragetHolder :type Object%20Object%20Reference))
  ;[1 1 1] Image
  (Http|RequestImageFunc url TragetHolder))

(event Custom|OnAwardsInfoCallback
  (params (AwardList :type Array%20of%20Struct%20Award%20Structures))
  ;[1 1 1] AwardsInfo
  (Utilities|FlowControl|Sequence
    (:then_0
      (if (stale Custom|RequestAwardsInfo IsCallUI?)
        (Default|OnAwardsInfoUpdated (Variables|Default|GetRef_WBP_AwardList) AwardList)))
    (:then_1
      (Default|UpdateAwardsList (Variables|Default|Getg_Drawer) AwardList)
      (for _array_element AwardList
        (CallFunction|RequestPoolQueue (.poolid _array_element))
        (CallFunction|RequestImageQueue (.awardimgurl _array_element))))))

(event Custom|OnPoolInfoCallback
  (params (PoolID :type String) (PlayserList :type Array%20of%20Struct%20Player%20Structures))
  ;[1 1 1] PoolInfo
  (Utilities|FlowControl|Sequence
    (:then_0
      (Default|UpdatePoolInfo (Variables|Default|Getg_Drawer) PoolID PlayserList)
      (if (stale Custom|RequestPoolInfo CallUI?)
        (Default|OnCharaInfoUpdated (Variables|Default|GetRef_WBP_AwardList) PlayserList)))
    (:then_1
      (for _array_element PlayserList
        (CallFunction|RequestImageQueue (.playerimgurl _array_element))))))

(event Custom|OnDrawedInfoCallback
  (params (Players :type Array%20of%20Struct%20Player%20Structures) (PoolName :type String) (AwardName :type String) (DrawNum :type Integer) (ResultCode :type String))
  ;[1 1 1] StartDraw
  (CallFunction|DrawedInfoCallbackandShowResultWBP PoolName AwardName DrawNum Players))

(event Custom|ResetServerStatus
  ;[1 1 1] ResetServerStatus
  (Http|RequestRestServerStatusFunc (delegate Custom|OnResetServerStatusCallback)))

(event Custom|OnResetServerStatusCallback
  ;[1 1 1] ResetServerStatus
  (CallFunction|RequestAwardsInfo true))

(event Custom|RequestPoolQueue
  (params (PoolID :type String%20%28by%20ref%29))
  ;[1 1 1] RequestPoolQueue
  (Utilities|FlowControl|Sequence
    (:then_0
      (Utilities|Array|AddUnique (Variables|Default|GettmpPoolRequestQueue) PoolID))
    (:then_1
      (Utilities|FlowControl|DoOnce false
        (:Completed
          (bind _returnvalue (Utilities|Time|SetTimerbyEvent (delegate Custom|PoolRequestQueue) 0.03 true)))))))

(fn ConstructionScript
  (Utilities|FlowControl|Sequence
    (:then_0
      (Utilities|SetupUserSetting))
    (:then_1
      (bind _returnvalue (Game|ConstructObjectfromClass "/Game/YearEndParty21/Blueprints/DrawerHttpHandler/BPO_Drawer.BPO_Drawer_C" self))
      (Variables|Default|Setg_Drawer _returnvalue))
    (:then_2
      (bind _outactors (Actor|GetAllActorswithTag "SpawnPoint"))
      (Variables|Default|Setg_SpawnFX (.AsBP%20Drawer%20Players (Utilities|Casting|CastToBP_DrawerPlayers (Utilities|Array|Get(acopy) _outactors)))))))

(fn CreateRequestHandler
  (bind _returnvalue (Game|ConstructObjectfromClass "/Game/YearEndParty21/Blueprints/DrawerHttpHandler/BP_HttpHandle.BP_HttpHandle_C" self))
  (return _returnvalue))

(fn RequestAwardsInfoFunc
  (params (事件 :type Delegate%20%28by%20ref%29))
  (Utilities|FlowControl|Sequence
    (:then_0
      (bind _newhttphandler (Http|CreateRequestHandler))
      (LocalVariables|SettmpHttpHandler _newhttphandler))
    (:then_1
      (EventDispatchers|BindEventtoAwardsInfoEvent (LocalVariables|GettmpHttpHandler) 事件))
    (:then_2
      (Default|RequestAwardsInfo (LocalVariables|GettmpHttpHandler)))))

(fn RequestImageFunc
  (params (url :type String) (TragetHolder :type Object%20Object%20Reference))
  (Utilities|FlowControl|Sequence
    (:then_0
      (bind _newhttphandler (Http|CreateRequestHandler))
      (LocalVariables|SettmpHttpHandler _newhttphandler))
    (:then_1
      (EventDispatchers|BindEventtoImageDownEvent (LocalVariables|GettmpHttpHandler) (EventDispatchers|CreateEvent :!event OnImageDownloaded)))
    (:then_2
      (Default|RequestDownImage (LocalVariables|GettmpHttpHandler) url TragetHolder (.Value (Utilities|Map|Find (Variables|Http|Getg_DownloadTex2d) url)))
      (return (LocalVariables|GettmpHttpHandler)))))

(fn OnImageDownloaded
  (params (url :type String) (tex2d :type Texture%202D%20Dynamic%20Object%20Reference))
  (Utilities|Map|Add (Variables|Http|Getg_DownloadTex2d) url tex2d))

(fn RequestPoolInfoFunc
  (params (pool_id :type String) (事件 :type Delegate%20%28by%20ref%29))
  (Utilities|FlowControl|Sequence
    (:then_0
      (bind _newhttphandler (Http|CreateRequestHandler))
      (LocalVariables|SettmpHttpHandler _newhttphandler))
    (:then_1
      (EventDispatchers|BindEventtoPlayerPoolEvent (LocalVariables|GettmpHttpHandler) 事件))
    (:then_2
      (Default|RequestPoolInfo (LocalVariables|GettmpHttpHandler) pool_id))))

(fn RequestStartDrawFunc
  (params (PoolID :type String) (AwardName :type String) (DrawNum :type Integer) (事件 :type Delegate%20%28by%20ref%29))
  (Utilities|FlowControl|Sequence
    (:then_0
      (bind _newhttphandler (Http|CreateRequestHandler))
      (LocalVariables|SettmpHttpHandler _newhttphandler))
    (:then_1
      (EventDispatchers|BindEventtoDrawedEvent (LocalVariables|GettmpHttpHandler) 事件))
    (:then_2
      (Default|RequestDraw (LocalVariables|GettmpHttpHandler) PoolID AwardName DrawNum))))

(fn RequestRestServerStatusFunc
  (params (事件 :type Delegate%20%28by%20ref%29))
  (Utilities|FlowControl|Sequence
    (:then_0
      (bind _newhttphandler (Http|CreateRequestHandler))
      (LocalVariables|SettmpHttpHandler _newhttphandler))
    (:then_1
      (EventDispatchers|BindEventtoResetedServerStatusEvent (LocalVariables|GettmpHttpHandler) 事件))
    (:then_2
      (Default|RequestResetServerStatus (LocalVariables|GettmpHttpHandler)))))

(fn ShowHideUI
  (params (WBP :type User%20Widget%20Object%20Reference) (IsShow? :type Boolean) (IsDebugMoving? :type Boolean))
  (bind _returnvalue (Game|GetPlayerController 0))
  (if IsShow?
    (UserInterface|Viewport|AddtoViewport WBP 0)
    (Input|SetInputModeUIOnly _returnvalue WBP "DoNotLock")
    (Variables|/Script/Engine.PlayerController|SetbShowMouseCursor _returnvalue true)
    (else
      (Widget|RemovefromParent WBP)
      (if IsDebugMoving?
        (Input|SetInputModeGameOnly _returnvalue)
        (else
          (Input|SetInputModeUIOnly _returnvalue 0 "LockOnCapture")))
      (Variables|/Script/Engine.PlayerController|SetbShowMouseCursor _returnvalue false))))

(fn GetCacheImagewithURL
  (params (Key :type String%20%28by%20ref%29))
  (return (.Value (Utilities|Map|Find (Variables|Http|Getg_DownloadTex2d) Key))))

(fn BacktoMainUI
  (CallFunction|RequestAwardsInfo true)
  (CallFunction|ShowHideUI (Variables|Default|GetRef_WBP_AwardList) false false))

(fn RequesCheckAnimationStatusFunc
  (params (事件 :type Delegate%20%28by%20ref%29))
  (Utilities|FlowControl|Sequence
    (:then_0
      (bind _newhttphandler (Http|CreateRequestHandler))
      (LocalVariables|SettmpHttpHandler _newhttphandler))
    (:then_1
      (EventDispatchers|BindEventtoCheckDrawStatusEvent (LocalVariables|GettmpHttpHandler) 事件))
    (:then_2
      (Default|RequestCheckAnimationStatus (LocalVariables|GettmpHttpHandler)))))

(fn DrawedInfoCallbackandShowResultWBP
  (params (PoolID :type String) (AwardName :type String) (LastDrawNum :type Integer) (PlayersInfo :type Array%20of%20Struct%20Player%20Structures))
  (Utilities|FlowControl|Sequence
    (:then_0
      (bind (_savedlastdrawawardinfo _savedlastdrawedplayerinfo) (Default|SetupLastDrawInfo (Variables|Default|Getg_Drawer) PoolID AwardName LastDrawNum PlayersInfo (Variables|Http|Getg_DownloadTex2d))))
    (:then_1
      (bind _returnvalue (UserInterface|CreateWidget "/Game/YearEndParty21/WBP/WBP_ResultInfo.WBP_ResultInfo_C"))
      (bind _output_get (Variables|Default|SetRef_WBP_ResultInfo _returnvalue))
      (Default|OnDrawEndUpdated _output_get _savedlastdrawawardinfo _savedlastdrawedplayerinfo)
      (UserInterface|Viewport|AddtoViewport _output_get 0))))

(fn ResetAnimationStatus
  (bind _ref_wbp_resultinfo (Variables|Default|GetRef_WBP_ResultInfo))
  (Utilities|FlowControl|Sequence
    (:then_0
      (Utilities|IsValid _ref_wbp_resultinfo
        (:Is%20Valid
          (Widget|RemovefromParent _ref_wbp_resultinfo))))
    (:then_1
      (Default|ResetStatus (Variables|Default|Getg_SpawnFX)))))