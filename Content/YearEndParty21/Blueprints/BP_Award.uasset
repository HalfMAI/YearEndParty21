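; BP_Award is an award display actor for the YearEndParty21 content, showing a WBP_Award widget in the world.
; SetupAwardInfo passes an image URL and award name to that widget.
; OnScaleUp plays a timeline that drives the widget component's world scale; OnEndAndDestory reverses it, then destroys the actor after a short delay.
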(event Custom|OnScaleUp
  (bind _scale (Timeline|ScaleUp Play)
    (:Update
      (Transformation|SetWorldScale3D (Variables|Default|GetWidget) (Math|Conversions|ToVector(Float) _scale)))))

(event Custom|OnEndAndDestory
  (Utilities|String|Reverse (Variables|Default|GetScaleUp))
  (Utilities|FlowControl|Delay 3.0)
  (Actor|DestroyActor))

(event EventBeginPlay)

(event Collision|EventActorBeginOverlap
  (params (OtherActor :type Actor%20Object%20Reference)))

(event EventTick
  (params (DeltaSeconds :type Float%20%28single-precision%29)))

(fn ConstructionScript)

(fn SetupAwardInfo
  (params (AwardImgURL :type String) (AwardName :type Text))
  (bind _aswbp_award (Utilities|Casting|CastToWBP_Award (UserInterface|GetWidget (Variables|Default|GetWidget))))
  (Default|SetupAwardInfo _aswbp_award AwardImgURL AwardName))