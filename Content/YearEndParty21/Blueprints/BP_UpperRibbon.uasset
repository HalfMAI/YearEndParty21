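; BP_UpperRibbon is an effect actor for YearEndParty21 that emits the NS_RibbonTop Niagara ribbon effect.
; On BeginPlay it spawns a batch of auto-release pooled systems attached to its root at the actor's transform, storing each in an array.
; When the actor is destroyed, it deactivates every stored system.
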(event EventBeginPlay
  (for _index (range 0 15)
    (bind _returnvalue (Niagara|SpawnSystemAttached "/Game/YearEndParty21/Effects/NS_RibbonTop.NS_RibbonTop" (Variables|Default|GetDefaultSceneRoot) "None" (Transformation|GetActorLocation) (Transformation|GetActorRotation) "KeepWorldPosition" true true "AutoRelease"))
    (Utilities|Array|AddUnique (Variables|Default|GettmpNSArray) _returnvalue)))

(event Collision|EventActorBeginOverlap
  (params (OtherActor :type Actor%20Object%20Reference)))

(event EventTick
  (params (DeltaSeconds :type Float%20%28single-precision%29)))

(event EventDestroyed
  (|CallParentFunction)
  (for _array_element (Variables|Default|GettmpNSArray)
    (Components|Activation|Deactivate _array_element)))

(fn ConstructionScript)