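; Year-end party prize-draw actor that stages a spinning cloud of player actors and presents the drawn winners.
; StartSpawn merges winners with the pool by player number, shuffles, then timer-spawns attached BP_Players in batches while rotation speeds up.
; Ending events batch-move players, reveal BP_Award with FX and an FOV change, then play end animations, polling until all are destroyed to signal completion.
; A separate event spawns winners one by one with burst FX.
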(event Custom|OnNeedSpawn
  (bind _returnvalue (Math|Random|RandomUnitVector))
  (bind _spawnrange (Variables|SpawnControl|GetSpawnRange))
  (bind _playerinfoneedtospawn (Variables|Default|GetPlayerInfoNeedToSpawn))
  (bind _spawnheight (Variables|SpawnControl|GetSpawnHeight))
  (bind _playerinfoneedtospawn_2 (Variables|Default|GetPlayerInfoNeedToSpawn))
  (bind _returnvalue_2 (Utilities|Array|Length _playerinfoneedtospawn_2))
  (bind _output (Utilities|Array|Get(acopy) _playerinfoneedtospawn))
  (bind (_playername _playerno _playerimgurl _holdingaward) (Utilities|Struct|BreakStruct_Player _output))
  (bind _returnvalue_3 (Math|Conversions|ToFloat(Integer) _returnvalue_2))
  (bind _returnvalue_4 (/ _returnvalue_3 1e+02))
  (bind _returnvalue_5 (Math|Float|Clamp(Float) _returnvalue_4 0.7))
  (bind _returnvalue_6 (* _spawnrange _returnvalue_5))
  (bind _returnvalue_7 (Math|Float|Truncate _returnvalue_6))
  (bind _returnvalue_8 (* _returnvalue _returnvalue_7))
  ;[1 1 1] Spawn
  (if (Variables|Default|GetIsPlayingStopAnimation?)
    (Utilities|Time|ClearandInvalidateTimerbyHandle (stale Custom|StartSpawn _returnvalue) :!label _label)
    (elif (<= (Utilities|Array|Length (Variables|Default|GetPlayerInfoNeedToSpawn)) 0)
      (goto _label)
      (else
        (Utilities|FlowControl|ForLoopwithBreak 0 10 :!label _label_2
          (:LoopBody
            (if (<= _returnvalue_2 0)
              (goto _label_2 Break)
              (elif false
                (if (Math|Random|RandomBool)
                  (Utilities|Array|RemoveItem (Variables|Default|GetPlayerInfoNeedToSpawn) _output)
                  (else
                    (bind _value (Default|GetCacheImagewithURL (Variables|Default|GetREF_GM_Party) _playerimgurl :!label _label_3))
                    (bind _returnvalue_9 (Game|SpawnActorfromClass "/Game/YearEndParty21/Blueprints/BP_Player.BP_Player_C" (Math|Transform|MakeTransform (+ (Transformation|GetActorLocation) (Math|Vector|MakeVector (.x _returnvalue_8) (.y _returnvalue_8) (Math|Random|RandomFloatinRange (* _spawnheight -1.0) _spawnheight))) (Math|Rotator|MakeRotator 0.0 0.0 (Math|Random|RandomFloatinRange 0.0 3.6e+02)) "1,1,1") "AlwaysSpawn" 0 (Utilities|Struct|MakeStruct_Player _playername _playerno _playerimgurl _holdingaward) _value (Math|Random|RandomFloatinRange 0.5 1.0) (Utilities|Array|ContainsItem (Variables|Default|GetDrawedPlayersInfo) _output) 0))
                    (Transformation|AttachActorToActor _returnvalue_9 self "None" "KeepWorld" "KeepWorld" "KeepWorld" true)
                    (Utilities|FlowControl|Sequence
                      (:then_0
                        (Utilities|Array|Add (Variables|Default|GetSpawnedPlayers) _returnvalue_9))
                      (:then_1
                        (Default|SetupTracePoint _returnvalue_9 (Variables|Default|GetDefaultSceneRoot))
                        (Utilities|Array|RemoveItem (Variables|Default|GetPlayerInfoNeedToSpawn) _output)))))
                (else
                  (goto _label_3))))))))))

(event Custom|StartSpawn
  (params (PlayerInfoNeedToSpawn :type Array%20of%20Struct%20Player%20Structures) (DrawedPlayersInfo :type Array%20of%20Struct%20Player%20Structures) (DrawAwardInfo :type Struct%20Award%20Structure))
  (bind (_drawedplayersinfo _playerinfoneedtospawn _ref_gm_party _spawnedplayers _isplayingstopanimation_ _spawndrawedplayeranimationendevent _spawnrange _spawndrawedplayertime _spawnheight _rotspeedinit) (Utilities|GetClassDefaults "BP_DrawerPlayers_C"))
  ;[1 1 1] Start
  (CallFunction|ResetStatus)
  (Utilities|FlowControl|Sequence
    (:then_0
      (bind _output_get (Variables|Default|SetDrawedPlayersInfo DrawedPlayersInfo))
      (Utilities|Array|Shuffle _output_get))
    (:then_1
      (bind _resultplayerinfoneedtospawn (CallFunction|CombineNeedtoSpawn PlayerInfoNeedToSpawn DrawedPlayersInfo))
      (bind _output_get_2 (Variables|Default|SetPlayerInfoNeedToSpawn _resultplayerinfoneedtospawn))
      (Utilities|Array|Shuffle _output_get_2))
    (:then_2
      (Variables|Default|SetCurrentDrawedAwardInfo DrawAwardInfo))
    (:then_3
      (Utilities|FlowControl|Sequence
        (:then_0
          ;;[1 1 1] Init
          (Variables|Default|SetREF_GM_Party (.AsGM%20Party (Utilities|Casting|CastToGM_Party (Game|GetGameMode))))
          (Variables|Default|SetIsPlayingStopAnimation? _isplayingstopanimation_)
          (Variables|SpawnControl|SetRotSpeedInit _rotspeedinit)
          (Transformation|SetRelativeScale3D (Variables|Default|GetDefaultSceneRoot) "1.000000,1.000000,1.000000"))
        (:then_1
          (CallFunction|PreReadyAnimation))
        (:then_2
          (bind _returnvalue (Utilities|Time|SetTimerbyEvent (delegate Custom|OnNeedSpawn) 0.05 true)))))))

(event Custom|tmpCheckAllFinished
  ;[1 1 1] CheckAllPlayerFinished
  (Variables|Default|SettmpIsAllFinished false)
  (bind _array_element (Utilities|Array|ForEachLoopwithBreak (Variables|Default|GetSpawnedPlayers) :!label _label)
    (:LoopBody
      (if (Utilities|IsValid _array_element)
        (Variables|Default|SettmpIsAllFinished false)
        (goto _label Break)
        (else
          (Variables|Default|SettmpIsAllFinished true))))
    (:Completed
      (if (Variables|Default|GettmpIsAllFinished)
        (Utilities|Time|ClearandInvalidateTimerbyHandle (stale Custom|CheckAllFinished _returnvalue))
        (Default|CallSpawnDrawedPlayerAnimationEndEvent)))))

(event Custom|CheckAllFinished
  ;[1 1 1] CheckAllPlayerFinished
  (bind _returnvalue (Utilities|Time|SetTimerbyEvent (delegate Custom|tmpCheckAllFinished) 1.0 true)))

(event Custom|PlayFlyAnimation
  (bind _currentdrawedawardinfo (Variables|Default|GetCurrentDrawedAwardInfo))
  (Utilities|FlowControl|Sequence
    (:then_0
      (Niagara|SpawnSystematLocation "/Game/YearEndParty21/Effects/NS_OcOut.NS_OcOut" (Transformation|GetActorLocation) "0, 0, 0" "1.000000,1.000000,1.000000" true true "AutoRelease" false)
      (bind _alpha (Timeline|ChangeFOV Play)
        (:Update
          (Variables|/Script/Engine.PlayerCameraManager|SetDefaultFOV (Game|GetPlayerCameraManager 0) (Math|Float|Lerp 9e+01 95.0 _alpha)))))
    (:then_1
      (bind _returnvalue (Game|SpawnActorfromClass "/Game/YearEndParty21/Blueprints/BP_Award.BP_Award_C" (Math|Transform|MakeTransform "5000.000000, 0, 0" "0,-180.000000, 0" "1,1,1") "AlwaysSpawn" 0 0))
      (Default|SetupAwardInfo _returnvalue (.awardimgurl _currentdrawedawardinfo) (Utilities|Text|ToText(String) (.awardname _currentdrawedawardinfo)))
      (Default|OnScaleUp _returnvalue))
    (:then_2
      (for _array_element (Variables|Default|GetSpawnedPlayers)
        (bind _asbp_player (Utilities|Casting|CastToBP_Player _array_element))
        (Default|ChangeFlyAngle _asbp_player)))))

(event Custom|PreReadyAnimation
  ;[1 1 1] PreReadyAni
  (Utilities|FlowControl|Sequence
    (:then_0
      (bind _speedup (Timeline|SpeedUp Play)
        (:Update
          (Variables|SpawnControl|SetRotSpeedInit (Math|Float|Lerp (Variables|SpawnControl|GetRotSpeedInit) (Variables|SpawnControl|GetRotSpeedMax) _speedup)))))
    (:then_1
      (bind _scale (Timeline|ScaleDown Play)
        (:Update
          (Transformation|SetWorldScale3D (Variables|Default|GetDefaultSceneRoot) _scale))))
    (:then_2
      (Utilities|FlowControl|Delay 1.0) ; Delay for spin up
      (bind _returnvalue (Utilities|Time|SetTimerbyEvent (delegate Custom|tmpSpawnFX) 0.2 true)))))

(event Custom|PlayPreEndAnimtion
  ;[1 1 1] PlayPreEndAnimation
  (Variables|Default|SetIsPlayingStopAnimation? true)
  (Utilities|Array|Shuffle (Variables|Default|GetSpawnedPlayers))
  (Variables|Default|SettmpLoopIndex 0)
  (bind _returnvalue (Utilities|Time|SetTimerbyEvent (delegate Custom|tmpMoveEndPos) 0.05 true)))

(event Custom|tmpMoveEndPos
  (bind _spawnedplayers (Variables|Default|GetSpawnedPlayers))
  (bind _tmploopindex (Variables|Default|GettmpLoopIndex))
  ;[1 1 1] PlayPreEndAnimation
  (if (<= (Utilities|Array|Length (Variables|Default|GetSpawnedPlayers)) 0) ; Finish the Undrawed Players
    (Utilities|Time|ClearandInvalidateTimerbyHandle (stale Custom|PlayPreEndAnimtion _returnvalue) :!label _label)
    (Utilities|FlowControl|Sequence
      (:then_0
        (goto _label_2 Reset))
      (:then_1
        (Utilities|IsValid (stale _returnvalue)
          (:Is%20Valid
            (Components|Activation|SetActive (stale _returnvalue) false false))))
      (:then_2
        (Utilities|IsValid (stale _returnvalue) ; If is normal route
          (:Is%20Valid
            (Utilities|FlowControl|Delay 3.0) ; Wait for all player Animation End
          )
          (:Is%20Not%20Valid
            _))
        (CallFunction|PlayFlyAnimation)))
    (else
      (Utilities|FlowControl|Sequence
        (:then_0
          (Utilities|FlowControl|DoOnce false :!label _label_2
            (:Completed
              (bind _returnvalue (Niagara|SpawnSystematLocation "/Game/YearEndParty21/Effects/NS_Oc.NS_Oc" (Transformation|GetActorLocation) "0, 0, 0" "1.000000,1.000000,1.000000" true true "AutoRelease")))))
        (:then_1
          (for _index (range 0 20)
            (if (>= _tmploopindex (Utilities|Array|Length _spawnedplayers)) ; Finish the Undrawed Players
              (goto _label)
              (else
                (Default|MovetoEndLoaction (Utilities|Array|Get(acopy) _spawnedplayers _tmploopindex))
                (Math|Integer|IncrementInt (Variables|Default|GettmpLoopIndex))))))))))

(event Custom|tmpDoAbsoveAnimationE
  (bind _drawedplayersinfo (Variables|Default|GetDrawedPlayersInfo))
  (bind _output (Utilities|Array|Get(acopy) _drawedplayersinfo))
  (bind (_playername _playerno _playerimgurl _holdingaward) (Utilities|Struct|BreakStruct_Player _output))
  ;[1 1 1] SpawnDrawedPlayer_AbsoveAndOut
  (if (Utilities|Array|IsValidIndex _drawedplayersinfo)
    (bind _value (Default|GetCacheImagewithURL (Variables|Default|GetREF_GM_Party) _playerimgurl))
    (bind _returnvalue (Game|SpawnActorfromClass "/Game/YearEndParty21/Blueprints/BP_Player.BP_Player_C" (Math|Transform|MakeTransform (Transformation|GetActorLocation) "0, 0, 0" "1,1,1") "AlwaysSpawn" 0 (Utilities|Struct|MakeStruct_Player _playername _playerno _playerimgurl _holdingaward) _value 1.0 true 0))
    (Default|OnDrawedPlayerdAnimation _returnvalue)
    (Utilities|FlowControl|Sequence
      (:then_0
        (Niagara|SpawnSystematLocation "/Game/YearEndParty21/Effects/NS_Brust.NS_Brust" (Transformation|GetActorLocation) "0,180.000000, 0" "1.000000,1.000000,1.000000" true true "AutoRelease"))
      (:then_1
        (Utilities|Array|RemoveIndex _drawedplayersinfo)))
    (else
      (Utilities|Time|ClearandInvalidateTimerbyHandle (stale Custom|SpawnDrawedPlayer_AbsoveAndOut _returnvalue))
      (Utilities|FlowControl|Delay 2.0)
      (Default|CallSpawnDrawedPlayerAnimationEndEvent))))

(event Custom|SpawnDrawedPlayer_AbsoveAndOut
  ;[1 1 1] SpawnDrawedPlayer_AbsoveAndOut
  (bind _returnvalue (Utilities|Time|SetTimerbyEvent (delegate Custom|tmpDoAbsoveAnimationE) (Variables|SpawnControl|GetSpawnDrawedPlayerTime) true)) ; Spawn Drawed Player
)

(event Custom|PlayDrawedPlayerAnimation
  ;[1 1 1] PlayDrawedPlayerAnimiation
  (Utilities|Array|Shuffle (Variables|Default|GetSpawnedPlayers))
  (Variables|Default|SettmpLoopIndex 0)
  (bind _returnvalue (Utilities|Time|SetTimerbyEvent (delegate Custom|tmpPlayEndAniEvent) 0.05 true)))

(event Custom|tmpSpawnFX
  (bind _spawnedplayers (Variables|Default|GetSpawnedPlayers))
  (bind _outitem (Utilities|Array|Random _spawnedplayers))
  ;[1 1 1] PreReadyAni
  (if (Variables|Default|GetIsPlayingStopAnimation?)
    (Utilities|Time|ClearandInvalidateTimerbyHandle (stale Custom|PreReadyAnimation _returnvalue))
    (else
      (Utilities|IsValid _outitem
        (:Is%20Valid
          (Default|SpawnFX _outitem))))))

(event Custom|tmpPlayEndAniEvent
  (bind _spawnedplayers (Variables|Default|GetSpawnedPlayers))
  (bind _tmploopindex (Variables|Default|GettmpLoopIndex))
  ;[1 1 1] PlayDrawedPlayerAnimiation
  (if (<= (Utilities|Array|Length (Variables|Default|GetSpawnedPlayers)) 0) ; Finish the Undrawed Players
    (Utilities|Time|ClearandInvalidateTimerbyHandle (stale Custom|PlayDrawedPlayerAnimation _returnvalue) :!label _label)
    (CallFunction|CheckAllFinished)
    (else
      (Utilities|FlowControl|Sequence
        (:then_0
          (for _index (range 0 10)
            (if (>= _tmploopindex (Utilities|Array|Length _spawnedplayers)) ; Finish all players
              (goto _label)
              (else
                (Default|EndAnimation (Utilities|Array|Get(acopy) _spawnedplayers _tmploopindex))
                (Math|Integer|IncrementInt (Variables|Default|GettmpLoopIndex))))))))))

(event EventTick
  (params (DeltaSeconds :type Float%20%28single-precision%29))
  ;[1 1 1] Tick
  (if (Variables|Default|GetIsPlayingStopAnimation?)
    _
    (else
      _))
  (Transformation|AddRelativeRotation (Variables|Default|GetDefaultSceneRoot) (Math|Rotator|MakeRotator 0.0 0.0 (* DeltaSeconds (Variables|SpawnControl|GetRotSpeedInit))) false false))

(fn ConstructionScript)

(fn ResetStatus
  (for _array_element (Variables|Default|GetSpawnedPlayers)
    (Utilities|IsValid _array_element
      (:Is%20Valid
        (Actor|DestroyActor _array_element))))
  (Utilities|Array|Clear (Variables|Default|GetSpawnedPlayers))
  (Utilities|Array|Clear (Variables|Default|GetPlayerInfoNeedToSpawn))
  (Utilities|Array|Clear (Variables|Default|GetDrawedPlayersInfo)))

(fn CombineNeedtoSpawn
  (params (PlayerInfoNeedToSpawn :type Array%20of%20Struct%20Player%20Structures) (DrawedPlayersInfo :type Array%20of%20Struct%20Player%20Structures))
  (LocalVariables|SettmpResultPlayerInfoNeedToSpawn DrawedPlayersInfo)
  (bind _array_element (Utilities|Array|ForEachLoopwithBreak PlayerInfoNeedToSpawn)
    (:LoopBody
      (LocalVariables|SettmpIsContainPlayer false)
      (bind _array_element_2 (Utilities|Array|ForEachLoopwithBreak DrawedPlayersInfo :!label _label)
        (:LoopBody
          (if (Utilities|Enum|Equal(Enum) (.PlayerNo (Utilities|Struct|BreakStruct_Player _array_element)) (.PlayerNo (Utilities|Struct|BreakStruct_Player _array_element_2)))
            (LocalVariables|SettmpIsContainPlayer true)
            (goto _label Break)))
        (:Completed
          (if (not (LocalVariables|GettmpIsContainPlayer))
            (Utilities|Array|Add (LocalVariables|GettmpResultPlayerInfoNeedToSpawn) _array_element)))))
    (:Completed
      (return (LocalVariables|GettmpResultPlayerInfoNeedToSpawn)))))