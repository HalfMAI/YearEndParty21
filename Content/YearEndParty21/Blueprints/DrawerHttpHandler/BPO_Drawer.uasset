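; Data object for a year-end party prize draw, holding the awards, pools, eligible players and last draw result.
; Updating the award list clears all cached data, including player lists, then rebuilds unique awards, award IDs (pool ID plus file name) and pool IDs.
; Player lists are replaced per pool name, with duplicates filtered out.
; The last draw stores award, count and winners, using placeholders for unused award fields.
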(fn ResetAwardsInfo
  (Utilities|Array|Clear (Variables|Default|Getg_AwardsInfo))
  (Utilities|Array|Clear (Variables|Default|Getg_AwardIDList))
  (Utilities|Array|Clear (Variables|Default|Getg_PoolList))
  (Utilities|Map|Clear (Variables|Default|Getg_PlayerList)))

(fn AddAwardInfo
  (params (NewAward :type Struct%20Award%20Structure%20%28by%20ref%29))
  (bind (_poolid _poolfilename) (Utilities|Struct|BreakStruct_Award NewAward))
  (Utilities|Array|AddUnique (Variables|Default|Getg_AwardsInfo) NewAward)
  (Utilities|Array|AddUnique (Variables|Default|Getg_AwardIDList) (Utilities|String|Append _poolid _poolfilename))
  (Utilities|Array|AddUnique (Variables|Default|Getg_PoolList) (.PoolID (Utilities|Struct|BreakStruct_Award NewAward))))

(fn UpdateAwardsList
  (params (AwardList :type Array%20of%20Struct%20Award%20Structures))
  (CallFunction|ResetAwardsInfo)
  (for _array_element AwardList
    (CallFunction|AddAwardInfo _array_element))
  (return))

(fn UpdatePoolInfo
  (params (PoolName :type String) (PoolPlayerList :type Array%20of%20Struct%20Player%20Structures))
  (Utilities|Map|Remove (Variables|Default|Getg_PlayerList) PoolName)
  (for _array_element PoolPlayerList
    (Utilities|Array|AddUnique (LocalVariables|GettmpPlayers) _array_element))
  (Utilities|Map|Add (Variables|Default|Getg_PlayerList) PoolName (Utilities|Struct|MakeStruct_Pool (Utilities|Array|MakeArray PoolName) (LocalVariables|GettmpPlayers)))
  (return))

(fn SetupLastDrawInfo
  (params (G%20Last%20Drawed%20Award%20Info%20Pool%20ID :type String) (G%20Last%20Drawed%20Award%20Info%20Award%20Name :type String) (g_LastDrawNum :type Integer) (g_LastDrawedPlayerInfo :type Array%20of%20Struct%20Player%20Structures))
  (Variables|Default|Setg_LastDrawedAwardInfo (Utilities|Struct|MakeStruct_Award G%20Last%20Drawed%20Award%20Info%20Pool%20ID "DefaultPoolFileName" G%20Last%20Drawed%20Award%20Info%20Award%20Name 0 "" 0 0 0))
  (Variables|Default|Setg_LastDrawNum g_LastDrawNum)
  (Variables|Default|Setg_LastDrawedPlayerInfo g_LastDrawedPlayerInfo))