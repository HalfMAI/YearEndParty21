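; HTTP handler for the year-end party prize draw, talking to the draw server through VaRest.
; Requests fetch awards, pool players and draw stage, start draws, reset server status and download images.
; Callbacks validate the code/payload response, build Player or Award structs and broadcast per-request dispatchers, while image downloads also notify the requester through BPI_HttpHandler.
; Completed requests fire OnRequestEnded, and ResetStatus unbinds result dispatchers and clears temporary player data.
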(event Custom|RequestAwardsInfo
  ;[1 1 1] RequestAwardsInfo
  (Class|VaRestSubsystem|CallURL (|VaRestSubsystem) (Utilities|String|Append (Variables|Paths|GetRequestPath) (Variables|Paths|GetGET_AwardInfoPath)) "GET" "x_www_form_urlencoded_url" 0 (EventDispatchers|CreateEvent :!event OnAwardsInfoCallback)))

(event Custom|RequestPoolInfo
  (params (PoolID :type String))
  ;[1 1 1] PoolInfo
  (Class|VaRestSubsystem|CallURL (|VaRestSubsystem) (Utilities|String|Append (Variables|Paths|GetRequestPath) (Variables|Paths|GetGET_PlayerPoolPath)) "GET" "x_www_form_urlencoded_url" (|MakeJson PoolID) (delegate Custom|OnRequestPoolInfoCallback)))

(event Custom|RequestDraw
  (params (PoolID :type String) (AwardName :type String) (DrawNum :type Integer))
  ;[1 1 1] StartDawring
  (Class|VaRestSubsystem|CallURL (|VaRestSubsystem) (Utilities|String|Append (Variables|Paths|GetRequestPath) (Variables|Paths|GetPOST_StartDrawPath)) "POST" "json" (|MakeJson PoolID AwardName (Utilities|String|ToString(Integer) DrawNum)) (delegate Custom|OnDrawCallback)))

(event Custom|RequestDownImage
  (params (url :type String) (InputObject :type Object%20Object%20Reference%20%28by%20ref%29))
  ;[1 1 1] DownloadImg
  (bind _returnvalue (CallFunction|EncodeURLFileName url))
  (bind _texture (|DownloadImage _returnvalue)
    (:OnSuccess
      (Default|CallImageDownEvent url _texture)
      (Utilities|FlowControl|Sequence
        (:then_0
          (CallFunction|CallonRequestEndFunc :!label _label))
        (:then_1
          (Utilities|IsValid InputObject
            (:Is%20Valid
              (bind _asbpi_http_handler (Utilities|Casting|CastToBPI_HttpHandler InputObject))
              (Default|OnImageDownloaded _asbpi_http_handler url _texture))))))
    (:OnFail
      (Development|PrintString 0 (Utilities|String|Append "DownloadFailed:" url) true true "(R=1.000000,G=0.000000,B=0.000000,A=1.000000)" 1e+01)
      (goto _label))))

(event Custom|OnRequestPoolInfoCallback
  (params (Request :type Va%20Rest%20Request%20JSON%20Object%20Reference))
  ;[1 1 1] PoolInfo
  (Utilities|FlowControl|Sequence
    (:then_0
      (bind (_code _msg _payload _rawstring) (Utilities|CheckIsResponseFormat Request)
        (:ResponseOK
          (if (Utilities|Enum|Equal(Enum) _code "1000")
            (Variables|Default|SettmpPoolPlayerJson (Class|VaRestJsonValue|AsArray _payload))
            (Utilities|FlowControl|Sequence
              (:then_0
                (Utilities|Array|Clear (Variables|Default|GettmpPoolPlayers)))
              (:then_1
                (for _array_element (Variables|Default|GettmpPoolPlayerJson)
                  (bind _struct_player (CallFunction|MakePlayer _array_element))
                  (Utilities|Array|AddUnique (Variables|Default|GettmpPoolPlayers) _struct_player)))
              (:then_2
                (Default|CallPlayerPoolEvent (stale Custom|RequestPoolInfo PoolID) (Variables|Default|GettmpPoolPlayers))))
            (else
              (Utilities|PrintErrorResponse _rawstring :!label _label))))
        (:ResponseFailed
          (goto _label))))
    (:then_1
      (CallFunction|CallonRequestEndFunc))))

(event Custom|OnDrawCallback
  (params (Request :type Va%20Rest%20Request%20JSON%20Object%20Reference))
  ;[1 1 1] StartDawring
  (Utilities|FlowControl|Sequence
    (:then_0
      (bind (_code _msg _payload _rawstring) (Utilities|CheckIsResponseFormat Request)
        (:ResponseOK
          (Utilities|FlowControl|Sequence
            (:then_0
              (Utilities|Array|Clear (Variables|Default|GettmpPoolPlayers)))
            (:then_1
              (switch string _code
                (:Default
                  (Utilities|PrintErrorResponse _rawstring :!label _label))
                (:1000
                  (for _array_element (Class|VaRestJsonValue|AsArray _payload)
                    (bind _struct_player (CallFunction|MakePlayer _array_element))
                    (Utilities|Array|AddUnique (Variables|Default|GettmpPoolPlayers) _struct_player))
                  (Default|CallDrawedEvent (Variables|Default|GettmpPoolPlayers) (stale Custom|RequestDraw PoolID) (stale Custom|RequestDraw AwardName) (stale Custom|RequestDraw DrawNum) _code))
                (:1001
                  (goto _label))
                (:1002
                  (goto _label))
                (:2000
                  (goto _label))))))
        (:ResponseFailed
          (goto _label))))
    (:then_1
      (CallFunction|CallonRequestEndFunc))))

(event Custom|RequestCheckAnimationStatus
  ;[1 1 1] CheckAnimationStatus
  (Class|VaRestSubsystem|CallURL (|VaRestSubsystem) (Utilities|String|Append (Variables|Paths|GetRequestPath) (Variables|Paths|GetGET_CheckDrawStage)) "GET" "x_www_form_urlencoded_url" 0 (delegate Custom|AnimationStatusCallback)))

(event Custom|AnimationStatusCallback
  (params (Request :type Va%20Rest%20Request%20JSON%20Object%20Reference))
  ;[1 1 1] CheckAnimationStatus
  (Utilities|FlowControl|Sequence
    (:then_0
      (bind (_code _msg _payload _rawstring) (Utilities|CheckIsResponseFormat Request)
        (:ResponseOK
          (if (Utilities|Enum|Equal(Enum) _code "1000")
            (bind _returnvalue (Class|VaRestJsonValue|AsObject _payload))
            (switch string (Class|VaRestJsonValue|AsString (Class|VaRestJsonObject|GetField _returnvalue "draw_stage"))
              (:Stage_Init
                (CallFunction|CallCheckDrawStatusEventFunc (Class|VaRestJsonValue|AsString (Class|VaRestJsonObject|GetField _returnvalue "draw_stage")) "" "" 0 (Utilities|Array|MakeArray "")))
              (:Stage_BeforeDraw
                (bind _returnvalue_2 (Class|VaRestJsonValue|AsObject (Class|VaRestJsonObject|GetField _returnvalue "last_draw_award_info") :!label _label))
                (bind _returnvalue_3 (Class|VaRestJsonValue|AsObject (Class|VaRestJsonObject|GetField _returnvalue_2 "drawed_award_info")))
                (Utilities|FlowControl|Sequence
                  (:then_0
                    (Utilities|Array|Clear (Variables|Default|GettmpPoolPlayers)))
                  (:then_1
                    (if (Class|VaRestJsonValue|IsNull (Class|VaRestJsonObject|GetField _returnvalue_2 "drawed_player_info"))
                      (CallFunction|CallCheckDrawStatusEventFunc (Class|VaRestJsonValue|AsString (Class|VaRestJsonObject|GetField _returnvalue "draw_stage")) (Class|VaRestJsonValue|AsString (Class|VaRestJsonObject|GetField _returnvalue_3 "draw_pool_id")) (Class|VaRestJsonValue|AsString (Class|VaRestJsonObject|GetField _returnvalue_3 "draw_award_name")) (Class|VaRestJsonValue|AsInt32 (Class|VaRestJsonObject|GetField _returnvalue_3 "draw_num")) (Utilities|Array|MakeArray "")) ; Don't have players
                      (else
                        (Variables|Default|SettmpPoolPlayerJson (Class|VaRestJsonValue|AsArray (Class|VaRestJsonObject|GetField _returnvalue_2 "drawed_player_info")))
                        (for _array_element (Variables|Default|GettmpPoolPlayerJson)
                          (bind _struct_player (CallFunction|MakePlayer _array_element))
                          (Utilities|Array|AddUnique (Variables|Default|GettmpPoolPlayers) _struct_player))
                        (CallFunction|CallCheckDrawStatusEventFunc (Class|VaRestJsonValue|AsString (Class|VaRestJsonObject|GetField _returnvalue "draw_stage")) (Class|VaRestJsonValue|AsString (Class|VaRestJsonObject|GetField _returnvalue_3 "draw_pool_id")) (Class|VaRestJsonValue|AsString (Class|VaRestJsonObject|GetField _returnvalue_3 "draw_award_name")) (Class|VaRestJsonValue|AsInt32 (Class|VaRestJsonObject|GetField _returnvalue_3 "draw_num")) (Variables|Default|GettmpPoolPlayers)) ; Have players
                      )))))
              (:Stage_StartDrawAnimation
                (goto _label))
              (:Stage_EndDrawAnimation
                (goto _label)))
            (else
              (Utilities|PrintErrorResponse _rawstring :!label _label_2))))
        (:ResponseFailed
          (goto _label_2))))
    (:then_1
      (CallFunction|CallonRequestEndFunc))))

(event Custom|RequestResetServerStatus
  ;[1 1 1] ResetServerStatus
  (Class|VaRestSubsystem|CallURL (|VaRestSubsystem) (Utilities|String|Append (Variables|Paths|GetRequestPath) (Variables|Paths|GetGET_ResetServerStatus)) "GET" "x_www_form_urlencoded_url" 0 (delegate Custom|OnResetServerStatus)))

(event Custom|OnResetServerStatus
  (params (Request :type Va%20Rest%20Request%20JSON%20Object%20Reference))
  ;[1 1 1] ResetServerStatus
  (Utilities|FlowControl|Sequence
    (:then_0
      (bind (_code _msg _payload _rawstring) (Utilities|CheckIsResponseFormat Request)
        (:ResponseOK
          (if (Utilities|Enum|Equal(Enum) _code "1000")
            (Default|CallResetedServerStatusEvent)
            (else
              (Utilities|PrintErrorResponse _rawstring :!label _label))))
        (:ResponseFailed
          (goto _label))))
    (:then_1
      (CallFunction|CallonRequestEndFunc))))

(fn MakePlayer
  (params (JsonObj :type Va%20Rest%20Json%20Value%20Object%20Reference%20%28by%20ref%29))
  (bind _returnvalue (Class|VaRestJsonValue|AsObject JsonObj))
  (if (Class|VaRestJsonObject|HasField _returnvalue "抽中奖品")
    (LocalVariables|SettmpHoldAwardInfo (Class|VaRestJsonValue|AsString (Class|VaRestJsonObject|GetField _returnvalue "抽中奖品")))
    (else
      (LocalVariables|SettmpHoldAwardInfo "未抽中")))
  (return (Utilities|Struct|MakeStruct_Player (Class|VaRestJsonValue|AsString (Class|VaRestJsonObject|GetField _returnvalue "player_name")) (Class|VaRestJsonValue|AsString (Class|VaRestJsonObject|GetField _returnvalue "player_no")) (Utilities|MakePlayerImgUrl (Class|VaRestJsonValue|AsString (Class|VaRestJsonObject|GetField _returnvalue "image_url"))) (LocalVariables|GettmpHoldAwardInfo))))

(fn OnAwardsInfoCallback
  (params (ResponseObject :type Va%20Rest%20Request%20JSON%20Object%20Reference))
  (Utilities|FlowControl|Sequence
    (:then_0
      (bind (_code _msg _payload _rawstring) (Utilities|CheckIsResponseFormat ResponseObject)
        (:ResponseOK
          (switch string _code
            (:Default
              (Utilities|PrintErrorResponse _rawstring))
            (:1000
              (Utilities|FlowControl|Sequence :!label _label
                (:then_0
                  (for _array_element (Class|VaRestJsonValue|AsArray _payload)
                    (bind _returnvalue (Class|VaRestJsonValue|AsObject _array_element))
                    (Utilities|Array|AddUnique (LocalVariables|GettmpAwardList) (Utilities|Struct|MakeStruct_Award (Class|VaRestJsonValue|AsString (Class|VaRestJsonObject|GetField _returnvalue "用户池")) (Class|VaRestJsonValue|AsString (Class|VaRestJsonObject|GetField _returnvalue "用户池列表名字")) (Class|VaRestJsonValue|AsString (Class|VaRestJsonObject|GetField _returnvalue "奖品名字")) (Class|VaRestJsonValue|AsInt32 (Class|VaRestJsonObject|GetField _returnvalue "奖品数目")) (Utilities|MakeAwardImgUrl (Class|VaRestJsonValue|AsString (Class|VaRestJsonObject|GetField _returnvalue "奖品图片名字"))) (Class|VaRestJsonValue|AsInt32 (Class|VaRestJsonObject|GetField _returnvalue "max_award_num")) (Class|VaRestJsonValue|AsInt32 (Class|VaRestJsonObject|GetField _returnvalue "award_num_left")) 0 (Utilities|Enum|Equal(Enum) (Class|VaRestJsonValue|AsString (Class|VaRestJsonObject|GetField _returnvalue "用户是否可抽中多奖品")) "是")))))
                (:then_1
                  (Default|CallAwardsInfoEvent (LocalVariables|GettmpAwardList)))))
            (:1001
              (goto _label))))))
    (:then_1
      (CallFunction|CallonRequestEndFunc))))

(fn EncodeURLFileName
  (params (InPath :type String))
  (bind _returnvalue (Class|VaRestLibrary|PercentEncode (Class|BlueprintPathsLibrary|GetCleanFilename InPath)))
  (return (Utilities|String|Append (Utilities|Paths|GetPath InPath) "/" _returnvalue)))

(fn MakeAnimationStatusResultValue)

(fn CallCheckDrawStatusEventFunc
  (params (CurDrawStage :type String) (DrawPoolID :type String) (DrawAwardName :type String) (DrawNum :type Integer) (DrawedPlayers :type Array%20of%20Struct%20Player%20Structures))
  (Default|CallCheckDrawStatusEvent CurDrawStage DrawPoolID DrawAwardName DrawNum DrawedPlayers))

(fn SetupRequestPath
  (params (RequestPath :type String))
  (Variables|Paths|SetRequestPath RequestPath))

(fn ResetStatus
  (Utilities|FlowControl|Sequence
    (:then_0
      (EventDispatchers|UnbindallEventsfromAwardsInfoEvent)
      (EventDispatchers|UnbindallEventsfromPlayerPoolEvent)
      (EventDispatchers|UnbindallEventsfromImageDownEvent)
      (EventDispatchers|UnbindallEventsfromDrawedEvent)
      (EventDispatchers|UnbindallEventsfromResetedServerStatusEvent)
      (EventDispatchers|UnbindallEventsfromCheckDrawStatusEvent))
    (:then_1
      (Utilities|Array|Clear (Variables|Default|GettmpPoolPlayerJson))
      (Utilities|Array|Clear (Variables|Default|GettmpPoolPlayers)))))

(fn CallonRequestEndFunc
  (Default|CallOnRequestEnded self))