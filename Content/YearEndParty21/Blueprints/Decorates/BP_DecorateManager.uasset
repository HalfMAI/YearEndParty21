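; Manager actor for the YearEndParty21 scene decorations, switching the Niagara star effect and held decorations between display and hide.
; On BeginPlay it activates the stars; a timeline drives their burst-angle parameter, played on hide and reversed on display.
; Hiding also uses a looping timer to animate out and destroy held decorations in small batches.
; Random box spawning with an exclusion zone and fog color shifting exist but are disconnected.
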(event Custom|HideDecorates
  ;[1 1 1] HidDecorates
  (Utilities|FlowControl|Sequence
    (:then_0
      (CallFunction|ShiftFogColor true)
      (CallFunction|ShiftStarSpeed true))
    (:then_1
      (bind _returnvalue (Utilities|Time|SetTimerbyEvent (delegate Custom|tmpHideDecorateEvent) 0.05 true)))))

(event Custom|tmpHideDecorateEvent
  (bind _holdingdecorates (Variables|Default|GetHoldingDecorates))
  (bind _output (Utilities|Array|Get(acopy) _holdingdecorates))
  ;[1 1 1] HidDecorates
  (for _index (range 0 5)
    (if (Utilities|Array|IsValidIndex _holdingdecorates)
      (Utilities|IsValid _output
        (:Is%20Valid
          (Default|ShowAnimaion _output false true))
        (:Is%20Not%20Valid
          _))
      (Utilities|Array|RemoveIndex _holdingdecorates)
      (else
        (Utilities|Time|ClearandInvalidateTimerbyHandle (stale Custom|HideDecorates _returnvalue))))))

(event Custom|DisplayDecorates
  (CallFunction|ShiftFogColor false)
  (CallFunction|ShiftStarSpeed false)
  (CallFunction|SetStarShow true))

(event Custom|ShiftFogColor
  (params (IsDispareColor? :type Boolean)))

(event Custom|ShiftStarSpeed
  (params (IsReduceAngle? :type Boolean))
  (if IsReduceAngle?
    (bind _alpha (Timeline|T_ShiftStarSpeed Play)
      (:Update
        (Niagara|SetNiagaraVariable(Float) (Variables|Default|GetNS_Star) "User.BurtAngleAlpha" _alpha)))
    (else
      (Timeline|T_ShiftStarSpeed Reverse))))

(event EventBeginPlay
  ;[1 1 1] BeginPlay
  (CallFunction|DisplayDecorates))

(fn ConstructionScript)

(fn RandomSpawnDecorate
  (params (SpawnNum :type Integer) (SpawnClass :type BP%20Decorate%20Base%20Class%20Reference))
  (bind _spawnbox (Variables|Default|GetSpawnBox))
  (bind _excluebox (Variables|Default|GetExclueBox))
  (for _index (range 0 SpawnNum)
    (bind _output_get (LocalVariables|SettmpPoint (Math|Random|RandomPointinBoundingBox (Transformation|GetWorldLocation _spawnbox) (Components|Box|GetScaledBoxExtent _spawnbox))))
    (if (not (Math|Geometry|IsPointinBox _output_get (Transformation|GetWorldLocation _excluebox) (Components|Box|GetScaledBoxExtent _excluebox)))
      (bind _returnvalue (Game|SpawnActorfromClass SpawnClass (Math|Transform|MakeTransform _output_get (Math|Rotator|MakeRotator 0.0 0.0 (Math|Random|RandomFloatinRange -3e+01 3e+01)) (Math|Conversions|ToVector(Float) (Math|Random|RandomFloatinRange 1.0 2.0))) "AlwaysSpawn" 0 0))
      (Utilities|Array|Add (Variables|Default|GetHoldingDecorates) _returnvalue))))

(fn SetupFog
  (bind _outactors (Actor|GetAllActorswithTag "EnvFog"))
  (bind _asexponential_height_fog (Utilities|Casting|CastToExponentialHeightFog (Utilities|Array|Get(acopy) _outactors)))
  (Variables|Default|SetRef_EnvFog _asexponential_height_fog))

(fn SetStarShow
  (params (IsStarShow? :type Boolean))
  (Components|Activation|SetActive (Variables|Default|GetNS_Star) IsStarShow? false))