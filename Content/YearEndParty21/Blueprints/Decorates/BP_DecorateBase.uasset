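; BP_DecorateBase is a decoration actor, apparently a base for decorations, that animates its appearance and disappearance by scaling.
; When ShouldPlayAnimation is set, BeginPlay zeroes the root scale and plays the Scale timeline after a random sub-second delay, staggering the pop-ins.
; ShowAnimaion plays or reverses that timeline, which drives clamped uniform root scale and can destroy the actor when finished.
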(event Custom|ShowAnimaion
  (params (IsShow? :type Boolean) (DestoryAfterFinished? :type Boolean))
  (if IsShow?
    (bind _scale (Timeline|Scale PlayFromStart)
      (:Update
        (Transformation|SetWorldScale3D (Variables|Default|GetDefaultSceneRoot) (Math|Conversions|ToVector(Float) (Math|Float|Clamp(Float) _scale))))
      (:Finished
        (if DestoryAfterFinished?
          (Actor|DestroyActor))))
    (else
      (Timeline|Scale ReverseFromEnd))))

(event EventBeginPlay
  (if (Variables|Default|GetShouldPlayAnimation?)
    (Transformation|SetWorldScale3D (Variables|Default|GetDefaultSceneRoot) "0, 0, 0")
    (Utilities|FlowControl|Delay (Math|Random|RandomFloatinRange 0.0 1.0))
    (Components|Timeline|PlayfromStart (Variables|Default|GetScale))))

(event Collision|EventActorBeginOverlap
  (params (OtherActor :type Actor%20Object%20Reference)))

(event EventTick
  (params (DeltaSeconds :type Float%20%28single-precision%29)))

(fn ConstructionScript)