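; Player card actor for a party prize draw, showing a participant's downloaded image, with name and number revealed only for the winner.
; On spawn it spins and pops in and out at shifting positions around a center, settling after two seconds.
; The end sequence scatters it around TracePoint, then the winner glows and flies toward the camera, while others dim, shrink and destroy themselves.
; SpawnFX attaches a throttled Niagara card splash.
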(event Custom|OnDrawedPlayerdAnimation
  (bind _returnvalue (Game|GetPlayerCameraManager 0))
  (bind _returnvalue_2 (Transformation|GetActorLocation))
  (bind _returnvalue_3 (Camera|GetCameraLocation _returnvalue))
  (bind _returnvalue_4 (+ _returnvalue_3 "0,-7.500000, 0"))
  (bind _returnvalue_5 (- _returnvalue_4 _returnvalue_2))
  ;[1 1 1] PlayDrawedPlayerAnimation
  (Variables|Default|SetIsPlayingEndAnimation true)
  (CallFunction|SetupTextDisplay false false)
  (Variables|Default|SetTargetLocation (+ _returnvalue_2 (* (Class|KismetMathLibrary|RandomUnitVectorinEllipticalConeinDegrees _returnvalue_5 7.0 1.0) (* (Math|Vector|VectorLength _returnvalue_5) 1.1))))
  (Variables|Default|SetStartLocation (Transformation|GetActorLocation))
  (bind _speed (Timeline|ToFront PlayFromStart)
    (:Update
      (Transformation|SetWorldLocation (Variables|Default|GetScene) (Math|Vector|Lerp(Vector) (Variables|Default|GetStartLocation) (Variables|Default|GetTargetLocation) _speed) false false))
    (:Finished
      (Utilities|FlowControl|Delay 1.0)
      (Actor|DestroyActor))))

(event Custom|MoveToEndLoactionAndDispare
  (bind _returnvalue (Math|Random|RandomFloatinRange -1e+02 1e+02))
  (bind _scene (Variables|Default|GetScene))
  (bind _trace_point (Variables|Default|GetTrace%20Point))
  (bind _returnvalue_2 (Transformation|GetWorldLocation _trace_point))
  ;[1 1 1] MoveToEndLoactionAndDispare
  (Variables|Default|SetIsPlayingEndAnimation true)
  (Transformation|DetachFromActor "KeepWorld" "KeepWorld" "KeepWorld")
  (Components|MoveComponentTo _scene (+ (Math|Random|RandomPointinBoundingBox _returnvalue_2 "200.000000,50.000000,10.000000") (* (Math|Random|RandomUnitVector) 1e+02)) "0, 0, 0" true true (Math|Random|RandomFloatinRange 0.5 2.0) true)
  (Components|MoveComponentTo _scene _returnvalue_2 "0, 0, 0" true true (Math|Random|RandomFloatinRange 0.2 0.5) true)
  (Utilities|FlowControl|Delay (Math|Random|RandomFloatinRange 1.0 2.0))
  (Components|MoveComponentTo (Variables|Default|GetScene) (+ (Transformation|GetWorldLocation (Variables|Default|GetTrace%20Point)) (Math|Vector|MakeVector _returnvalue (Math|Random|RandomFloatinRange -3e+02 3e+02) _returnvalue)) "0, 0, 0" true true (Math|Random|RandomFloatinRange 0.1 0.3) true)
  (if (Variables|Default|GetIsCurrentDrawedAndGotAward?)
    (CallFunction|SetupMaterialEmissiveAmount 1.0)
    (Utilities|FlowControl|Delay (Math|Random|RandomFloatinRange 1.0 3.0))
    (CallFunction|OnDrawedPlayerdAnimation)
    (else
      (CallFunction|SetupMaterialEmissiveAmount 0.1)
      (Utilities|FlowControl|Delay (Math|Random|RandomFloatinRange 0.2 1.0))
      (CallFunction|DoEndAnimationandDestory))))

(event Custom|ScaleUpOrDown
  (bind _scene (Variables|Default|GetScene))
  (bind _returnvalue (Transformation|GetWorldLocation _scene))
  ;[1 1 1] ScaleAni
  (bind _isa (Utilities|FlowControl|FlipFlop)
    (:A
      _)
    (:B
      _))
  (Utilities|FlowControl|DoOnce false :!label _label
    (:Completed
      (if _isa
        (bind (_direction _scale) (Timeline|ScaleUpMainScene Play)
          (:Update
            (Transformation|SetRelativeScale3D (Variables|Default|GetPlane) (Math|Conversions|ToVector(Float) (Math|Float|Clamp(Float) _scale))))
          (:Finished
            (if (not (Variables|Default|GetIsPlayingEndAnimation))
              (Utilities|FlowControl|Sequence
                (:then_0
                  (switch Utilities|FlowControl|Switch|SwitchonETimelineDirection _direction
                    (:Backward
                      (Utilities|IsValid _scene
                        (:Is%20Valid
                          (Transformation|SetWorldLocation _scene (Math|Vector|MakeVector (.x _returnvalue) (.y _returnvalue) (+ (Math|Random|RandomFloatinRange -5e+01 1e+02) (.z (Transformation|GetWorldLocation (Variables|Default|GetTrace%20Point))))) false false)
                          (Transformation|SetRelativeLocation _scene (Math|Vector|RotateVector (Variables|/Script/Engine.SceneComponent|GetRelativeLocation _scene) (Math|Rotator|MakeRotator 0.0 0.0 (Math|Random|RandomFloatinRange 45.0 135.0))) false false))))))
                (:then_1
                  (Utilities|FlowControl|Delay (Math|Random|RandomFloatinRange 0.1 1.0))
                  (goto _label Reset))))))
        (else
          (Timeline|ScaleUpMainScene Reverse))))))

(event Custom|RandomScaleUpOrDown
  ;[1 1 1] Begin Play Setup
  (if (not (Variables|Default|GetIsPlayingEndAnimation))
    (CallFunction|ScaleUporDown)))

(event Custom|SpawnFX
  (Utilities|SpawnFXMacro))

(event Custom|DoEndAnimationAndDestory
  ;[1 1 1] DoUnDrawedPlayerDestoryEndAnimation
  (bind _scale_ (Timeline|ScaleDown Play)
    (:Update
      (Transformation|SetWorldScale3D (Variables|Default|GetScene) (Math|Conversions|ToVector(Float) _scale_)))
    (:Finished
      (Development|SetHiddeninGame (Variables|Default|GetScene) true true)
      (Actor|DestroyActor))))

(event EventBeginPlay
  (bind _tex2d (Variables|Default|GetTex2d))
  ;[1 1 1] Begin Play Setup
  (Utilities|FlowControl|Sequence
    (:then_0
      (CallFunction|InitPlayerInfo)
      (bind _returnvalue (Rendering|Material|CreateDynamicMaterialInstance (Variables|Default|GetPlane) 0 "/Game/YearEndParty21/Blueprints/M_CardSprite.M_CardSprite" "None" :!class /Script/Engine.PrimitiveComponent))
      (Variables|Default|SetSMMaterial _returnvalue)
      (if (Variables|Default|GetIsCurrentDrawedAndGotAward?)
        (CallFunction|SetupTextDisplay false true)
        (else
          (CallFunction|SetupTextDisplay true true))))
    (:then_1
      (Utilities|IsValid _tex2d
        (:Is%20Valid
          (CallFunction|SetupTexture _tex2d))
        (:Is%20Not%20Valid
          (bind _asgm_party (Utilities|Casting|CastToGM_Party (Game|GetGameMode)))
          (Default|RequestImage _asgm_party (.PlayerImgURL (Utilities|Struct|BreakStruct_Player (Variables|Default|GetPlayerInfo))) self))))
    (:then_2
      (CallFunction|ScaleUporDown))
    (:then_3
      (bind _returnvalue_2 (Utilities|Time|SetTimerbyEvent (delegate Custom|RandomScaleUpOrDown) 1.0 true 0.0 1.0)))
    (:then_4
      (Utilities|FlowControl|Delay 2.0)
      (Actor|Tick|SetActorTickEnabled false)
      (Utilities|Time|ClearandInvalidateTimerbyHandle _returnvalue_2)
      (Audio|Components|Audio|Play (Variables|Default|GetScaleUpMainScene)))))

(event EventTick
  (params (DeltaSeconds :type Float%20%28single-precision%29))
  ;[1 1 1] Tick
  (if (not (Variables|Default|GetIsPlayingEndAnimation))
    (Transformation|AddRelativeRotation (Variables|Default|GetScene) (Math|Rotator|MakeRotator 0.0 0.0 (* DeltaSeconds 2e+02)) false false)))

(event EventOnImageDownloaded
  (params (srcURL :type String) (tex2d :type Texture%202D%20Dynamic%20Object%20Reference))
  ;[1 1 1] On ImageDownloaded
  (CallFunction|SetupTexture tex2d))

(fn ConstructionScript)

(fn InitPlayerInfo
  (bind _playerinfo (Variables|Default|GetPlayerInfo))
  (Utilities|FlowControl|Sequence
    (:then_0
      (Rendering|Components|TextRender|SetText (Variables|Default|GettName) (Utilities|Text|ToText(String) (.playername _playerinfo))))
    (:then_1
      (Rendering|Components|TextRender|SetText (Variables|Default|GettNo) (Utilities|Text|ToText(String) (.playerno _playerinfo))))))

(fn SetupTextDisplay
  (params (IsDestory? :type Boolean) (IsHidden? :type Boolean))
  (bind _textsparent (Variables|Default|GetTextsParent))
  (if IsDestory?
    (Components|DestroyComponent (Variables|Default|GetTextsParent))
    (Components|DestroyComponent (Variables|Default|GettNo))
    (Components|DestroyComponent (Variables|Default|GettName))
    (else
      (Utilities|IsValid _textsparent
        (:Is%20Valid
          (Development|SetHiddeninGame _textsparent IsHidden? true))))))

(fn SetupTracePoint
  (params (TracePoint :type Scene%20Component%20Object%20Reference))
  (Variables|Default|SetTrace%20Point TracePoint))

(fn SetupTexture
  (params (Texture :type Texture%20Object%20Reference))
  (Rendering|Material|SetTextureParameterValue (Variables|Default|GetSMMaterial) "MainImg" Texture)
  (Utilities|FlowControl|Sequence
    (:then_1
      (return))))

(fn SetupMaterialEmissiveAmount
  (params (EmissiveAmount :type Float%20%28single-precision%29))
  (Rendering|Material|SetScalarParameterValue (Variables|Default|GetSMMaterial) "EmissiveAmount" EmissiveAmount :!class /Script/Engine.MaterialInstanceDynamic))