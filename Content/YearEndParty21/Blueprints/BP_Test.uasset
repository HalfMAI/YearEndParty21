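; Test actor that samples a component's surface with a grid of line traces over its bounding box.
; DoTraceOnBoundingBox splits the Y-Z face of the bounds into small square cells and fires a complex Visibility trace along X through each, with debug drawing.
; Hit points and normals are returned as arrays.
; BeginPlay calls it without a component, so as written it only prints an invalid-component message.
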(event EventBeginPlay
  (CallFunction|DoTraceonBoundingBox))

(event Collision|EventActorBeginOverlap
  (params (OtherActor :type Actor%20Object%20Reference)))

(event EventTick
  (params (DeltaSeconds :type Float%20%28single-precision%29)))

(fn ConstructionScript)

(fn DoTraceonBoundingBox
  (params (Component :type Scene%20Component%20Object%20Reference))
  (bind (_origin _boxextent) (Collision|GetComponentBounds Component))
  (bind _boxextent_2 (Collision|GetComponentBounds Component))
  (LocalVariables|SettmpSquareBoxSize 5.0)
  (Utilities|IsValid Component
    (:Is%20Valid
      (for _index (range 0 (Math|Float|Round (* (* 2 (/ (.y _boxextent_2) (LocalVariables|GettmpSquareBoxSize))) (* 2 (/ (.z _boxextent_2) (LocalVariables|GettmpSquareBoxSize))))))
        (bind (_outhit _returnvalue) (Collision|LineTraceByChannel (Math|Vector|MakeVector (+ (.x _origin) 1e+02) (+ (- (+ (.y _origin) (* (LocalVariables|GettmpSquareBoxSize) 0.5)) (.y _boxextent)) (* (Math|Integer|%(Integer) _index (Math|Float|Round (* 2 (/ (.y _boxextent_2) (LocalVariables|GettmpSquareBoxSize))))) (LocalVariables|GettmpSquareBoxSize))) (+ (- (+ (.z _origin) (* (LocalVariables|GettmpSquareBoxSize) 0.5)) (.z _boxextent)) (* (/ _index (Math|Float|Round (* 2 (/ (.y _boxextent_2) (LocalVariables|GettmpSquareBoxSize))))) (LocalVariables|GettmpSquareBoxSize)))) (Math|Vector|MakeVector (+ (.x _origin) -1e+02) (+ (- (+ (.y _origin) (* (LocalVariables|GettmpSquareBoxSize) 0.5)) (.y _boxextent)) (* (Math|Integer|%(Integer) _index (Math|Float|Round (* 2 (/ (.y _boxextent_2) (LocalVariables|GettmpSquareBoxSize))))) (LocalVariables|GettmpSquareBoxSize))) (+ (- (+ (.z _origin) (* (LocalVariables|GettmpSquareBoxSize) 0.5)) (.z _boxextent)) (* (/ _index (Math|Float|Round (* 2 (/ (.y _boxextent_2) (LocalVariables|GettmpSquareBoxSize))))) (LocalVariables|GettmpSquareBoxSize)))) "TraceTypeQuery1" true 0 "ForDuration" false))
        (if _returnvalue
          (Utilities|Array|Add (LocalVariables|GettmpImpactPoint) (.impactpoint _outhit))
          (Utilities|Array|Add (LocalVariables|GettmpImpactNormal) (.impactnormal _outhit))))
      (return (LocalVariables|GettmpImpactPoint) (LocalVariables|GettmpImpactNormal)))
    (:Is%20Not%20Valid
      (Development|PrintString "Component is Not Valid"))))